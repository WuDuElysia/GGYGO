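; Player character Blueprint for Pyrios, adding ability-input resource preparation, stylized-render key light binding and turn-back foley.
; BeginPlay starts ability input/render resource preparation outside dedicated servers once the pawn extension accepts it.
; It binds StylizedRenderComponent to the sole GGYGO.KeyLight-tagged DirectionalLight, otherwise logging and deactivating any valid component.
; Movement updates only read the TurnBack phase, playing one attached foley sound per entry into Turning.
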(event `self.ReceiveBeginPlay`
  (bind _stylizedrendercomponent (`self.StylizedRenderComponent`))
  (bind _returnvalue (`KismetSystemLibrary.GetPathName` self))
  (bind _returnvalue_2 (`GGYGOPawnExtensionComponent.FindPawnExtensionComponent` self))
  ; 项目配置：TurnBack 起始播放第一段衣甲声一次；原版触发条件未知。
  ; 监听原生移动完成事件，读取 CMC 相位；不驱动运动。RunOut 后重入 Turning 可再次播放。
  (add `self.OnCharacterMovementUpdated` self (delegate `OnCharacterMovementUpdated_0`))
  (if (not (`KismetSystemLibrary.IsDedicatedServer` self))
    (bind _returnvalue_3 (`GGYGONiagaraMaterialPreparation.CreateForSystemAssets` _returnvalue_2 self (`self.AbilityInputRenderSystems`)))
    (bind _returnvalue_4 (`GGYGOPawnExtensionComponent.SetAbilityInputResourcePreparation` _returnvalue_2 _returnvalue_3))
    (if _returnvalue_4
      (`GGYGONiagaraMaterialPreparation.Start` _returnvalue_3)))
  (if (`KismetSystemLibrary.IsValid` _stylizedrendercomponent)
    (bind _outactors (`GameplayStatics.GetAllActorsWithTag` self "GGYGO.KeyLight"))
    (bind _returnvalue_5 (`KismetArrayLibrary.Array_Length` _outactors))
    (if (== _returnvalue_5 1)
      (bind _output (`|GetArrayItem` _outactors))
      (bind `_as定向光源` (cast `DirectionalLight` _output)
        (:`then`
          (if (`KismetSystemLibrary.IsValid` `_as定向光源`)
            (set `GGYGOCharacterRenderComponent.KeyLight` `_as定向光源` _stylizedrendercomponent)
            (`ActorComponent.Activate` _stylizedrendercomponent false)
            (else
              (`ActorComponent.Deactivate` _stylizedrendercomponent)
              (bind _returnvalue_6 (`KismetSystemLibrary.GetPathName` _output))
              (`KismetSystemLibrary.PrintString` self (`KismetStringLibrary.Concat_StrStr` (`KismetStringLibrary.Concat_StrStr` _returnvalue " [主灯绑定拒绝] Tag=GGYGO.KeyLight 唯一候选不是有效 DirectionalLight：") _returnvalue_6) false))))
        (:`CastFailed`
          (`ActorComponent.Deactivate` _stylizedrendercomponent)
          (`KismetSystemLibrary.PrintString` self (`KismetStringLibrary.Concat_StrStr` (`KismetStringLibrary.Concat_StrStr` _returnvalue " [主灯绑定拒绝] Tag=GGYGO.KeyLight 唯一候选不是有效 DirectionalLight：") _returnvalue_6) false)))
      (else
        (`ActorComponent.Deactivate` _stylizedrendercomponent)
        (`KismetSystemLibrary.PrintString` self (`KismetStringLibrary.Concat_StrStr` _returnvalue (`KismetStringLibrary.BuildString_Int` "" " [主灯绑定拒绝] Tag=GGYGO.KeyLight 实际数量=" _returnvalue_5 "；要求恰好一个，不绑定。")) false)))
    (else
      (`KismetSystemLibrary.PrintString` self (`KismetStringLibrary.Concat_StrStr` _returnvalue " [主灯绑定拒绝] 缺少有效组件 StylizedRenderComponent；Tag=GGYGO.KeyLight") false))))

(event `OnCharacterMovementUpdated_0` :!signature `self.OnCharacterMovementUpdated`
  (params (DeltaSeconds :type "Float (single-precision)") (OldLocation :type "Vector Structure") (OldVelocity :type "Vector Structure"))
  ; 项目配置：TurnBack 起始播放第一段衣甲声一次；原版触发条件未知。
  ; 监听原生移动完成事件，读取 CMC 相位；不驱动运动。RunOut 后重入 Turning 可再次播放。
  (if (== (`GGYGOCharacterMovementComponent.GetTurnBackPhase` (`self.GetGGYGOMovementComponent` self)) 1)
    (if (not (`self.bWasTurnBackTurningForFoley`))
      (set `self.bWasTurnBackTurningForFoley` true)
      (`GameplayStatics.SpawnSoundAttached` "/Game/Characters/Player/Pyrios/Audio/TurnBack/SW_Pyrios_Foley_Pyrois_TurnBack.SW_Pyrios_Foley_Pyrois_TurnBack" (`self.Mesh`) "None" (0.0 0.0 0.0) (struct) "KeepRelativeOffset" true 1.0 1.0 0.0 null null))
    (else
      (set `self.bWasTurnBackTurningForFoley` false))))

(fn `UserConstructionScript`)